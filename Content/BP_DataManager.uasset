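; BP_DataManager turns the player's position into a lookup in WomenDataTable, selecting data by country and year.
; Each Tick, player X picks one of ten CountryArray entries and player Z picks a year from 2007 to 2022, both clamped.
; The two form a Country_Year row name, and a found row is stored in CurrentRow, which otherwise keeps its previous value.
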(event EventTick
  (params (DeltaSeconds :type Float%20%28single-precision%29))
  (bind _returnvalue (Game|GetPlayerCharacter 0))
  (bind _returnvalue_2 (Transformation|GetActorLocation _returnvalue))
  (bind (_x _y _z) (Math|Vector|BreakVector _returnvalue_2))
  (bind _returnvalue_3 (Utilities|GetDataTableRow (Variables|Default|GetWomenDataTable) (Utilities|String|StringToName (Utilities|String|Append (Utilities|String|Append (Utilities|Array|Get(acopy) (Variables|Default|GetCountryArray%20) (Math|Conversions|ToInteger(Byte) (Class|KismetMathLibrary|ClampInt64 (Class|KismetMathLibrary|ToInt64(Float) (/ _x 4e+02)) 0 9))) "_") (Utilities|String|ToString(Integer) (Class|KismetMathLibrary|ClampInt64 (Class|KismetMathLibrary|ToInt64(Float) (+ (/ _z 2e+02) 2007.0)) 2007 2022)))))
    (:then
      (Variables|Default|SetCurrentRow%20%20 _returnvalue_3))))

(fn ConstructionScript)