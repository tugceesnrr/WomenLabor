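; BP_ShadowCharacter is a shadow actor that trails the player pawn, which it caches on BeginPlay.
; Each Tick it eases its location toward the player's position plus a fixed world-space Y offset, without sweeping.
; It also interpolates forward vectors toward the player's facing, but that interpolation has no DeltaTime input, unlike the location one.
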(event EventBeginPlay
  (Variables|Default|SetPlayerRef (Game|Player|GetPlayerPawn 0)))

(event EventTick
  (params (DeltaSeconds :type Float%20%28single-precision%29))
  (Transformation|SetActorLocation (Math|Interpolation|VInterpTo (Transformation|GetActorLocation) (+ (Transformation|GetActorLocation (Variables|Default|GetPlayerRef)) "0.000000,-500.000000,0.000000") DeltaSeconds 5.0) false false)
  (Transformation|SetActorRotation (Math|Conversions|RotationFromXVector (Math|Interpolation|VInterpTo (Math|Rotator|GetRotationXVector (Transformation|GetActorRotation)) (Math|Rotator|GetRotationXVector (Transformation|GetActorRotation (Variables|Default|GetPlayerRef))) 0.0 5.0))))

(fn ConstructionScript)