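; Fog visualization actor that follows the player pawn and drives a Niagara fog effect from yearly average data.
; Each tick it snaps to the pawn, and once the pawn is at least 50 units from the last recorded spot it advances the year counter.
; That year's row in the FogYillikOrtalama table supplies a Rating, inversely remapped to set the Niagara FogDensity parameter, alongside a debug print.
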(event EventBeginPlay
  (Variables|Default|SetLastLocation%20 (Transformation|GetActorLocation)))

(event EventTick
  (params (DeltaSeconds :type Float%20%28single-precision%29))
  (bind _returnvalue (Math|Float|Truncate DeltaSeconds))
  (bind _returnvalue_2 (Game|Player|GetPlayerPawn _returnvalue))
  (bind _returnvalue_3 (Transformation|GetActorLocation _returnvalue_2))
  (Transformation|SetActorLocation (+ _returnvalue_3 "-0.000000,0.000000,0.000000") false false)
  (if (>= (Math|Vector|Distance(Vector) _returnvalue_3 (Variables|Default|GetLastLocation%20)) 5e+01)
    (Variables|Default|SetLastLocation%20 _returnvalue_3)
    (Variables|Default|SetCurrentYear (+ (Variables|Default|GetCurrentYear) 1))
    (bind _returnvalue_4 (Utilities|GetDataTableRow "/Game/Fog/FogYillikOrtalama.FogYillikOrtalama" (Utilities|String|StringToName (Utilities|String|ToString(Integer) (Variables|Default|GetCurrentYear))))
      (:then
        (Development|PrintString "Hello" true true "(R=0.000000,G=0.660000,B=1.000000,A=1.000000)" (Math|Float|MapRangeClamped (Math|Conversions|ToFloat(Integer) (.rating (Utilities|Struct|BreakS_Bech _returnvalue_4))) 0.0 3.0 1.5e+02 3e+01))
        (Niagara|SetNiagaraVariable(Float) (Variables|Default|GetNiagara) "User.FogDensity" (Math|Float|MapRangeClamped (Math|Conversions|ToFloat(Integer) (.rating (Utilities|Struct|BreakS_Bech _returnvalue_4))) 0.0 3.0 1.5e+02 3e+01))))))

(fn ConstructionScript)